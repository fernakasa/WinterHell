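; Game instance Blueprint that owns the save game, persisting the player's checkpoint, spawn transform and current level.
; Init loads SaveGame_BP from the slot or creates one; SavePlayerData updates and writes it, and ClearSaveData deletes the slot.
; LoadLevelData teleports the FirstPersonCharacter to the saved transform, aligns control rotation and re-enables checkpoint collision, without using LevelName.
; LoadPlayerData is an empty stub.
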(event `self.ReceiveInit`
  (bind _returnvalue (`GameplayStatics.DoesSaveGameExist` (`self.SaveSlotName`)))
  (if _returnvalue
    (bind _returnvalue_2 (`GameplayStatics.LoadGameFromSlot` (`self.SaveSlotName`)))
    (bind _assave_game_bp (cast `/Game/SaveSystem/Blueprints/SaveGame_BP` _returnvalue_2)
      (:`then`
        (set `self.SaveGameData` _assave_game_bp)
        (`KismetSystemLibrary.PrintString` "Partida cargada"))
      (:`CastFailed`
        (`KismetSystemLibrary.PrintString` "Fallo al cargar partida")))
    (else
      (bind _returnvalue_3 (`GameplayStatics.CreateSaveGameObject` "/Game/SaveSystem/Blueprints/SaveGame_BP.SaveGame_BP_C"))
      (set `self.SaveGameData` _returnvalue_3)
      (`KismetSystemLibrary.PrintString` "Partida creada"))))

(fn `ClearSaveData`
  (bind _returnvalue (`GameplayStatics.DeleteGameInSlot` (`self.SaveSlotName`)))
  (if _returnvalue
    (`KismetSystemLibrary.PrintString` "Archivo Borrado")))

(fn `LoadLevelData`
  (params (LevelName :type String))
  (bind _returnvalue (`GameplayStatics.GetPlayerCharacter` 0))
  (bind _spawnplace (`/Game/SaveSystem/Blueprints/SaveGame_BP.SpawnPlace` (`self.SaveGameData`)))
  (cast `/Game/FirstPersonBP/Blueprints/Character/FirstPersonCharacter` _returnvalue)
  (`Actor.K2_SetActorTransform` _returnvalue _spawnplace false false)
  (`Controller.SetControlRotation` (`GameplayStatics.GetPlayerController` 0) (`KismetMathLibrary.MakeRotator` 0.0 (.pitch (.rotation _spawnplace)) (.yaw (.rotation _spawnplace))))
  (`Actor.SetActorEnableCollision` (`/Game/SaveSystem/Blueprints/SaveGame_BP.CheckPointEnable` (`self.SaveGameData`)) true))

(fn `LoadPlayerData`)

(fn `SavePlayerData`
  (params (checkpoint :type "/Game/FirstPersonBP/Blueprints/Triggers/CheckPoints/CheckPoint_BP Object Reference") (spawn :type "Transform Structure") (level :type String))
  (bind _savegamedata (`self.SaveGameData`))
  (set `/Game/SaveSystem/Blueprints/SaveGame_BP.CheckPointEnable` checkpoint _savegamedata)
  (set `/Game/SaveSystem/Blueprints/SaveGame_BP.SpawnPlace` spawn _savegamedata)
  (set `/Game/SaveSystem/Blueprints/SaveGame_BP.CurrentLevel` level _savegamedata)
  (bind _returnvalue (`GameplayStatics.SaveGameToSlot` _savegamedata (`self.SaveSlotName`)))
  (if _returnvalue
    (`KismetSystemLibrary.PrintString` "Guardado")))